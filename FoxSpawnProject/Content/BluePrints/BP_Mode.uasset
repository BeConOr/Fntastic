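; BP_Mode is a setup Blueprint that creates the button UI and the hole and end point actors at game start.
; On BeginPlay it adds WBP_Buttons to the viewport, then spawns three BP_Hole and BP_EndPoint pairs spaced along X by HoleStep, with end points offset along Y.
; It hands each pair to the widget's First, Second and Third references, so the UI holds direct links to them.
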(event `self.ReceiveBeginPlay`
  (bind _returnvalue (`|GenericCreateObject` "/Game/BluePrints/WBP_Buttons.WBP_Buttons_C"))
  (bind _output_get (set `self.Buttons` _returnvalue))
  (`UserWidget.AddToViewport` _output_get 0)
  (`self.SpawnHoles`))

(fn `SpawnHoles`
  (bind _buttons (`self.Buttons`))
  (for _index (range 3)
    (bind _returnvalue (* _index (`self.HoleStep`)))
    (bind _returnvalue_2 (`|SpawnActorFromClass` "/Game/BluePrints/BP_Hole.BP_Hole_C" (`KismetMathLibrary.MakeTransform` (`KismetMathLibrary.MakeVector` _returnvalue)) "Undefined" "OverrideRootScale" null null))
    (bind _returnvalue_3 (`|SpawnActorFromClass` "/Game/BluePrints/BP_EndPoint.BP_EndPoint_C" (`KismetMathLibrary.MakeTransform` (`KismetMathLibrary.MakeVector` _returnvalue 2000.0)) "Undefined" "OverrideRootScale" null null))
    (switch `int` _index
      (:`0`
        (set `/Game/BluePrints/WBP_Buttons.FirstHole` _returnvalue_2 _buttons)
        (set `/Game/BluePrints/WBP_Buttons.FirstEndPoint` _returnvalue_3 _buttons))
      (:`1`
        (set `/Game/BluePrints/WBP_Buttons.SecondHole` _returnvalue_2 _buttons)
        (set `/Game/BluePrints/WBP_Buttons.SecondEndPoint` _returnvalue_3 _buttons))
      (:`2`
        (set `/Game/BluePrints/WBP_Buttons.ThirdHole` _returnvalue_2 _buttons)
        (set `/Game/BluePrints/WBP_Buttons.ThirdEndPoint` _returnvalue_3 _buttons)))))

(fn `UserConstructionScript`)